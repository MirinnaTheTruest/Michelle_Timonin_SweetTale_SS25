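; BP_LevelEnd is a level goal actor with a crown that spins slightly every tick.
; When BP_PuddingPrincess overlaps it, it shows the WBP_GameEnd widget, switches to UI-only input with a visible cursor and disables input on the princess.
; It then plays an end sound and fades out the music by taking the first AmbientSound actor found in the level.
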(event Collision|EventActorBeginOverlap
  (params (OtherActor :type Actor%20Object%20Reference))
  (bind _returnvalue (Game|GetPlayerController 0))
  ;[0.15 0.15 0.15 0.5] Shows Game End Screen
  (bind _asbp_pudding_princess (Utilities|Casting|CastToBP_PuddingPrincess OtherActor))
  (bind _returnvalue_2 (UserInterface|CreateWidget "/Game/MyGame/UI/WBP_GameEnd.WBP_GameEnd_C"))
  (UserInterface|Viewport|AddtoViewport _returnvalue_2 0)
  (Input|SetInputModeUIOnly _returnvalue 0 "DoNotLock" false)
  (Variables|/Script/Engine.PlayerController|SetbShowMouseCursor _returnvalue true)
  (Input|DisableInput _asbp_pudding_princess 0)
  (Audio|SpawnSoundatLocation "/Game/MyGame/Sound/S_GameEnd.S_GameEnd" "0, 0, 0" "0, 0, 0" 1.0 1.0 0.0 0 0)
  ;[0.15 0.15 0.15 0.5] Fades Out Music
  (bind _outactors (Actor|GetAllActorsOfClass "/Script/Engine.AmbientSound"))
  (Audio|Components|Audio|FadeOut (Variables|/Script/Engine.AmbientSound|GetAudioComponent (Utilities|Array|Get(acopy) _outactors)) 2.0 0.0 "Linear" :!class /Script/Engine.AudioComponent))

(event EventTick
  (params (DeltaSeconds :type Float%20%28single-precision%29))
  ;[0.15 0.15 0.15 0.5] Rotates Crown
  (Transformation|AddLocalRotation (Variables|Default|GetCrown) "0.000000,0.100000,0.000000" false false))

(fn ConstructionScript)