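; BP_Rope is a swingable rope with a cloud that BP_PuddingPrincess can grab and launch from.
; Its capsule overlap gives the character a rope reference, and attach parents it to the cable end, which swing forces push.
; Detaching launches the player forward and up, resets double jump and briefly limits rope collision to physics only.
; MoveRope runs a timeline sliding cable and cloud toward an end location; construction places both at the start.
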(event OnComponentEndOverlap(Capsule)
  (params (OverlappedComponent :type Primitive%20Component%20Object%20Reference) (OtherActor :type Actor%20Object%20Reference) (OtherComp :type Primitive%20Component%20Object%20Reference) (OtherBodyIndex :type Integer))
  ;[0.15 0.15 0.15 0.5] Attaching and Detaching when in Collision Box
  (bind _asbp_pudding_princess (Utilities|Casting|CastToBP_PuddingPrincess OtherActor))
  (Variables|/Game/MyGame/Character/BP_PuddingPrincess.BP_PuddingPrincess_C|SetCanAttachToRope _asbp_pudding_princess false)
  (Variables|/Game/MyGame/Character/BP_PuddingPrincess.BP_PuddingPrincess_C|SetRopeRef _asbp_pudding_princess 0))

(event OnComponentBeginOverlap(Capsule)
  (params (OverlappedComponent :type Primitive%20Component%20Object%20Reference) (OtherActor :type Actor%20Object%20Reference) (OtherComp :type Primitive%20Component%20Object%20Reference) (OtherBodyIndex :type Integer) (bFromSweep :type Boolean) (SweepResult :type Hit%20Result%20Structure%20%28by%20ref%29))
  ;[0.15 0.15 0.15 0.5] Attaching and Detaching when in Collision Box
  (bind _asbp_pudding_princess (Utilities|Casting|CastToBP_PuddingPrincess OtherActor))
  (Variables|/Game/MyGame/Character/BP_PuddingPrincess.BP_PuddingPrincess_C|SetCanAttachToRope _asbp_pudding_princess true)
  (Variables|/Game/MyGame/Character/BP_PuddingPrincess.BP_PuddingPrincess_C|SetRopeRef _asbp_pudding_princess self))

(event Custom|MoveRope
  (bind _end_location (Variables|Default|GetEnd%20Location))
  ;[0.15 0.15 0.15 0.5] Moves Rope once Triggered
  (bind _newtrack_0 (Timeline|RopeMovement Play)
    (:Update
      (Transformation|SetRelativeLocation (Variables|Default|GetCloud) (Math|Vector|Lerp(Vector) (Variables|Default|GetCloudLocation) _end_location _newtrack_0) false false)
      (Transformation|SetRelativeLocation (Variables|Default|GetCable) (Math|Vector|Lerp(Vector) (Variables|Default|GetCableLocation) _end_location _newtrack_0) false false))))

(event Custom|AttachToRope
  (params (Target%20Character :type BP%20Pudding%20Princess%20Object%20Reference))
  (bind _cableend (Variables|Default|GetCableEnd))
  (bind _returnvalue (Transformation|GetWorldLocation _cableend))
  ;[0.15 0.15 0.15 0.5] Attaching and Detaching
  (Transformation|AttachComponentToComponent Target%20Character (Variables|Default|GetCableEnd) "None" "KeepWorld" "KeepWorld" "KeepWorld" true)
  ;[0.15 0.15 0.15 0.5] correcting character Position
  (Transformation|SetActorLocation Target%20Character (+ (Math|Vector|MakeVector (.x _returnvalue) (.y _returnvalue) (- (.z _returnvalue) 2e+01)) (* (Transformation|GetActorForwardVector (Game|GetPlayerCharacter 0)) -2e+01)) false false))

(event Custom|DetachFromRope
  (params (Target%20Character :type BP%20Pudding%20Princess%20Object%20Reference))
  (bind _returnvalue (Game|GetPlayerCharacter 0))
  ;[0.15 0.15 0.15 0.5] Attaching and Detaching
  (Transformation|DetachFromActor Target%20Character "KeepWorld" "KeepWorld" "KeepWorld")
  ;[0.15 0.15 0.15 0.5] Not colliding with the Rope, what probably pushed me downwards before
  (Collision|SetCollisionEnabled (Variables|Default|GetCable) "PhysicsOnly")
  ;[0.15 0.15 0.15 0.5] Launch Character
  (Character|LaunchCharacter Target%20Character (+ (* (Transformation|GetActorForwardVector _returnvalue) 8e+02) (* (Transformation|GetActorUpVector _returnvalue) 5e+02)) true true)
  ;[0.15 0.15 0.15 0.5] Reset Double Jump
  (Pawn|Components|CharacterMovement|SetMovementMode (Variables|/Script/Engine.Character|GetCharacterMovement Target%20Character) "MOVE_Walking" 0)
  ;[0.15 0.15 0.15 0.5] enable collision
  (Utilities|FlowControl|Delay 1.0)
  (Collision|SetCollisionEnabled (Variables|Default|GetCable) "QueryAndPhysics"))

(event Custom|Add%20Swinging%20Force
  (params (Swinging%20Force :type Vector))
  ;[0.15 0.15 0.15 0.5] Rope Swinging Force
  (Physics|AddForce (Variables|Default|GetCableEnd) (* Swinging%20Force 6e+02) "None" true))

(event EventBeginPlay
  ;[0.15 0.15 0.15 0.5] Get Cables and Cloud location
  (Variables|Default|SetCableLocation (Variables|/Script/Engine.SceneComponent|GetRelativeLocation (Variables|Default|GetCable)))
  (Variables|Default|SetCloudLocation (Variables|/Script/Engine.SceneComponent|GetRelativeLocation (Variables|Default|GetCloud))))

(fn ConstructionScript
  (Transformation|SetRelativeLocation (Variables|Default|GetCable) (Variables|Default|GetStart%20Location) false false))