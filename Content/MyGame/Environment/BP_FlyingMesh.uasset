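; BP_FlyingMesh is an environment Blueprint that makes a static mesh hover by moving it up and down.
; The construction script applies a mesh and material set per instance.
; On BeginPlay, the Moving timeline starts at a random time so instances bob out of sync, and its track lerps the mesh's relative Z offset above and below the origin.
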(event EventBeginPlay
  ;[0.15 0.15 0.15 0.5] moving up and down
  ;;[0.15 0.15 0.15 0.5] Instances start at random Times
  (Components|Timeline|SetNewTime (Variables|Default|GetMoving) (Math|Random|RandomFloat))
  (bind _newtrack_0 (Timeline|Moving Play)
    (:Update
      (Transformation|SetRelativeLocation (Variables|Default|GetStaticMesh) (Math|Vector|Lerp(Vector) "0.000000,0.000000,10.000000" "0.000000,0.000000,-10.000000" _newtrack_0) false false))))

(fn ConstructionScript
  ;[0.15 0.15 0.15 0.5] Set mesh per instance
  (Components|StaticMesh|SetStaticMesh (Variables|Default|GetStaticMesh) (Variables|Default|GetMovingMesh))
  ;[0.15 0.15 0.15 0.5] Set material per instance
  (Rendering|Material|SetMaterial (Variables|Default|GetStaticMesh) 0 (Variables|Default|GetMeshMaterial)))